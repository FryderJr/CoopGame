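; BP_AdvancedAI is an AI-controlled pawn that runs the BT_AdvancedAI behavior tree and shows its health in a widget component.
; HealthComponent's change event refreshes the WBP_Health display and records when the pawn last took damage.
; Tick auto-heals the pawn in periodic steps once it has gone several seconds without damage, throttled by timestamps rather than timers.
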(event Custom|OnHealthChanged_Event_0
  (params (HealthComp :type S%20Health%20Component%20Object%20Reference) (Health :type Float%20%28single-precision%29) (HealthDelta :type Float%20%28single-precision%29) (DamageType :type Damage%20Type%20Object%20Reference) (InstigatedBy :type Controller%20Object%20Reference) (DamageCauser :type Actor%20Object%20Reference))
  (Utilities|FlowControl|Sequence
    (:then_0
      ;[1 1 1] Save last time pawn took damage
      (if (> HealthDelta 0.0)
        (Variables|Default|SetLastTimeDamaged (Utilities|Time|GetTimeSeconds))))
    (:then_1
      (CallFunction|DisplayHealth))))

(event EventBeginPlay
  (Utilities|FlowControl|Sequence
    (:then_0
      (CallFunction|DisplayHealth))
    (:then_1
      ;[1 1 1] Run Behaviour tree
      (AI|RunBehaviorTree (AI|GetAIController self) "/Game/AdvancedAI/BT_AdvancedAI.BT_AdvancedAI"))
    (:then_2
      (EventDispatchers|AssignOnHealthChanged (Variables|Default|GetHealthComponent) (delegate Custom|OnHealthChanged_Event_0)))))

(event EventTick
  (params (DeltaSeconds :type Float%20%28single-precision%29))
  ;[1 1 1] Auto heal
  (if (and (> (- (Utilities|Time|GetTimeSeconds) (Variables|Default|GetLastTimeDamaged)) 7.0) (> (- (Utilities|Time|GetTimeSeconds) (Variables|Default|GetLastTimeHealed)) 1.0))
    (Class|SHealthComponent|Heal (Variables|Default|GetHealthComponent) 1e+01)
    (Variables|Default|SetLastTimeHealed (Utilities|Time|GetTimeSeconds))))

(fn ConstructionScript)

(fn DisplayHealth
  (bind _aswbp_health (Utilities|Casting|CastToWBP_Health (UserInterface|GetUserWidgetObject (Variables|Default|GetWidget))))
  (Default|UpdateHealth _aswbp_health (Variables|/Script/CoopGame.SHealthComponent|GetHealth (Variables|Default|GetHealthComponent))))